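; Free-flying server pawn that looks and moves through Enhanced Input and switches a marker environment between zones.
; On BeginPlay it adds its mapping context and caches all BP_Zone actors plus the BP_AltEnvironmentWithMarkers actor.
; The action input steps through the zones, wrapping on an invalid entry, and moves that environment to the selected zone.
; Each Tick passes the root transform to SendClient or SendServer depending on authority.
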(event Custom|SendClient
  (params (A :type Transform%20%28by%20ref%29))
  (Transformation|SetWorldTransform (Variables|Default|GetDefaultSceneRoot) A false false))

(event Custom|SendServer
  (params (A :type Transform%20%28by%20ref%29))
  (Transformation|SetWorldTransform (Variables|Default|GetDefaultSceneRoot) A false false))

(event Custom|ZoneMove
  (params (타깃 :type Scene%20Component%20Object%20Reference) (NewLocation :type Vector))
  (Transformation|SetWorldLocation (Variables|/AntilatencySDK/Blueprints/Samples/Actors/BP_AltEnvironment.BP_AltEnvironment_C|GetDefaultSceneRoot (Variables|Default|GetMarker)) NewLocation false false))

(event Input|EnhancedActionEvents|EnhancedInputActionIA_Server_Up
  (params (ActionValue :type Vector%202D%20Structure) (ElapsedSeconds :type Float%20%28double-precision%29) (TriggeredSeconds :type Float%20%28double-precision%29) (InputAction :type Input%20Action%20Object%20Reference :default "/Game/M1/Input/IA_Server_Up.IA_Server_Up"))
  (bind _defaultsceneroot (Variables|Default|GetDefaultSceneRoot))
  (bind _returnvalue (Math|Vector|GetUpVector _defaultsceneroot))
  (Pawn|Input|AddMovementInput _returnvalue (.x ActionValue) false)
  (Pawn|Input|AddMovementInput _returnvalue (.y ActionValue) false))

(event Input|EnhancedActionEvents|EnhancedInputActionIA_Server_Action1
  (params (ActionValue :type Boolean) (ElapsedSeconds :type Float%20%28double-precision%29) (TriggeredSeconds :type Float%20%28double-precision%29) (InputAction :type Input%20Action%20Object%20Reference :default "/Game/M1/Input/IA_Server_Action1.IA_Server_Action1"))
  (:Started
    (if (!= (Variables|Default|GetZone%20Length) (Variables|Default|GetZone%20Count))
      (Math|Integer|IncrementInt (Variables|Default|GetZone%20Count)
        (:%20%20
          (Utilities|IsValid (Utilities|Array|Get(acopy) (Variables|Default|GetZone) (Variables|Default|GetZone%20Count))
            (:Is%20Valid
              _)
            (:Is%20Not%20Valid
              (Variables|Default|SetZone%20Count 0)))
          (Variables|Default|GetMarker
            (:then
              (CallFunction|ZoneMove 0 (Transformation|GetWorldLocation (Variables|/Game/M1/Main/BP_Zone.BP_Zone_C|GetDefaultSceneRoot (Utilities|Array|Get(acopy) (Variables|Default|GetZone) (Variables|Default|GetZone%20Count))))))
            (:else)))))))

(event Input|EnhancedActionEvents|EnhancedInputActionIA_Look
  (params (ActionValue :type Vector%202D%20Structure) (ElapsedSeconds :type Float%20%28double-precision%29) (TriggeredSeconds :type Float%20%28double-precision%29) (InputAction :type Input%20Action%20Object%20Reference :default "/Game/M1/Input/IA_Look.IA_Look"))
  (Pawn|Input|AddControllerYawInput (.x ActionValue))
  (Pawn|Input|AddControllerPitchInput (* (.y ActionValue) -1.0)))

(event Input|EnhancedActionEvents|EnhancedInputActionIA_Server_Forward
  (params (ActionValue :type Vector%202D%20Structure) (ElapsedSeconds :type Float%20%28double-precision%29) (TriggeredSeconds :type Float%20%28double-precision%29) (InputAction :type Input%20Action%20Object%20Reference :default "/Game/M1/Input/IA_Server_Forward.IA_Server_Forward"))
  (bind _defaultsceneroot (Variables|Default|GetDefaultSceneRoot))
  (bind _returnvalue (Math|Vector|GetForwardVector _defaultsceneroot))
  (Pawn|Input|AddMovementInput _returnvalue (.x ActionValue) false)
  (Pawn|Input|AddMovementInput _returnvalue (.y ActionValue) false))

(event Input|EnhancedActionEvents|EnhancedInputActionIA_Server_Right
  (params (ActionValue :type Vector%202D%20Structure) (ElapsedSeconds :type Float%20%28double-precision%29) (TriggeredSeconds :type Float%20%28double-precision%29) (InputAction :type Input%20Action%20Object%20Reference :default "/Game/M1/Input/IA_Server_Right.IA_Server_Right"))
  (bind _defaultsceneroot (Variables|Default|GetDefaultSceneRoot))
  (bind _returnvalue (Math|Vector|GetRightVector _defaultsceneroot))
  (Pawn|Input|AddMovementInput _returnvalue (.x ActionValue) false)
  (Pawn|Input|AddMovementInput _returnvalue (.y ActionValue) false))

(event EventBeginPlay
  (Utilities|FlowControl|Sequence
    (:then_0
      (bind _asbp_pc (Utilities|Casting|CastToBP_PC (Game|GetPlayerController 0)))
      (Utilities|IsValid (PlayerController|LocalPlayerSubsystems|GetEnhancedInputLocalPlayerSubsystem _asbp_pc)
        (:Is%20Valid
          (Input|AddMappingContext (PlayerController|LocalPlayerSubsystems|GetEnhancedInputLocalPlayerSubsystem _asbp_pc) "/Game/M1/Input/IMC_ServerPawn.IMC_ServerPawn" 0 "(bIgnoreAllPressedKeysUntilRelease=True,bForceImmediately=False,bNotifyUserSettings=False)"))))
    (:then_1
      (bind _outactors (Actor|GetAllActorsOfClass "/Game/M1/Main/BP_Zone.BP_Zone_C"))
      (if (not (Utilities|Array|IsEmpty _outactors))
        (bind _output_get (Variables|Default|SetZone _outactors))
        (Variables|Default|SetZone%20Length (Utilities|Array|Length _output_get))
        (bind _returnvalue (Actor|GetActorOfClass "/AntilatencySDK/Blueprints/Samples/Actors/BP_AltEnvironmentWithMarkers.BP_AltEnvironmentWithMarkers_C"))
        (Utilities|IsValid _returnvalue
          (:Is%20Valid
            (Variables|Default|SetMarker _returnvalue)))))))

(event EventTick
  (params (DeltaSeconds :type Float%20%28single-precision%29))
  (bind _defaultsceneroot (Variables|Default|GetDefaultSceneRoot))
  (bind _returnvalue (Transformation|GetWorldTransform _defaultsceneroot))
  (Networking|SwitchHasAuthority
    (:Authority
      (CallFunction|SendClient _returnvalue))
    (:Remote
      (CallFunction|SendServer _returnvalue))))

(fn ConstructionScript)

(fn ChangZone)