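; BP_PC is a controller Blueprint that switches a non-VR user onto the BP_ServerPawn found in the level.
; On BeginPlay it checks whether a head-mounted display is enabled and prints the result.
; Without a headset, it unpossesses its current pawn and possesses the server pawn, provided that pawn is valid and not already player-controlled.
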(event EventBeginPlay
  (bind _output_get (Variables|Default|SetbHeadMountedDisplay? (Class|HeadMountedDisplayFunctionLibrary|IsHeadMountedDisplayEnabled)))
  (Development|PrintText (Utilities|Text|ToText(Boolean) _output_get) true true "(R=0.000000,G=0.660000,B=1.000000,A=1.000000)" 5.0)
  (if (not _output_get)
    (bind _returnvalue (Actor|GetActorOfClass "/Game/M1/System/BP_ServerPawn.BP_ServerPawn_C"))
    (Utilities|IsValid _returnvalue
      (:Is%20Valid
        (if (not (and (Class|Pawn|IsPawnControlled _returnvalue) (Pawn|IsPlayerControlled _returnvalue)))
          (Pawn|UnPossess)
          (Pawn|Possess _returnvalue))))))

(fn ConstructionScript)