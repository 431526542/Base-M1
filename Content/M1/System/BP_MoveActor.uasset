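; BP_MoveActor is an actor whose mesh component moves back and forth between two marker components, A and B.
; When IsMove is set at BeginPlay, it interpolates SM to A or B over RunningTime using MoveComponentTo.
; Each completed move toggles Index through a FlipFlop and calls Move, which loops back to start the next trip endlessly.
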(event Custom|Move
  (Components|MoveComponentTo (Variables|Default|GetSM) (select (Variables|Default|GetIndex) (Variables|/Script/Engine.SceneComponent|GetRelativeLocation (Variables|Default|GetB)) (Variables|/Script/Engine.SceneComponent|GetRelativeLocation (Variables|Default|GetA))) "0, 0, 0" false false (Variables|Default|GetRunning%20Time) false)
  (Utilities|FlowControl|FlipFlop
    (:A
      (Variables|Default|SetIndex true))
    (:B
      (Variables|Default|SetIndex false)))
  (CallFunction|Move))

(event EventBeginPlay
  (if (Variables|Default|GetIsMove?)
    (Components|MoveComponentTo (Variables|Default|GetSM) (select (Variables|Default|GetIndex) (Variables|/Script/Engine.SceneComponent|GetRelativeLocation (Variables|Default|GetB)) (Variables|/Script/Engine.SceneComponent|GetRelativeLocation (Variables|Default|GetA))) "0, 0, 0" false false (Variables|Default|GetRunning%20Time) false)
    (Utilities|FlowControl|FlipFlop
      (:A
        (Variables|Default|SetIndex true))
      (:B
        (Variables|Default|SetIndex false)))
    (CallFunction|Move)))

(fn ConstructionScript)