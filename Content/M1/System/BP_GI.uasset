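; BP_GI, likely the Game Instance, handles room entry and LAN multiplayer sessions.
; One event creates the room entry widget once, caches it and adds it to the viewport.
; CreateRoom2 starts a LAN session and, on success, opens Room_No2 as a listen server.
; EnterRoom joins a session from a passed-in search result, with no failure handling on either session call.
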(event Custom|informationAndRoomEntryAtStart
  (Utilities|IsValid (Variables|Default|GetWBP_RoomEnterAtStart)
    (:Is%20Valid
      _)
    (:Is%20Not%20Valid
      (bind _returnvalue (UserInterface|CreateWidget "/Game/M1/System/WBP_RoomEntryAtStart.WBP_RoomEntryAtStart_C" (Game|GetPlayerController 0)))
      (Variables|Default|SetWBP_RoomEnterAtStart _returnvalue)))
  (UserInterface|Viewport|AddtoViewport (Variables|Default|GetWBP_RoomEnterAtStart) 0))

(event Custom|EnterRoom
  (params (SearchResult :type Blueprint%20Session%20Result%20Structure%20%28by%20ref%29))
  (|JoinSession (Game|GetPlayerController 0) SearchResult))

(event Custom|CreateRoom2
  (|Session (Game|GetPlayerController 0) 20 true
    (:OnSuccess
      (Game|OpenLevel(byName) "Room_No2" true "listen"))))