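; VR pawn that drives head and body meshes from an Alt-tracked Oculus HMD camera and replicates them in multiplayer.
; A looping timer copies the camera transform to the head and its location and yaw to the body, skipping the copy while the camera sits at the environment marker.
; Non-authority instances send both transforms to the server, which multicasts them.
; The pawn destroys itself when unpossessed.
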(event Custom|Send%20Clients
  (params (Head :type Transform%20%28by%20ref%29) (Body :type Transform))
  ;[0.09375 0.09375 0.09375] Replicate
  (Transformation|SetWorldTransform (Variables|Default|GetCamera) Head false false)
  (Transformation|SetWorldTransform (Variables|Default|GetSM_Body) Body false false))

(event Custom|Send%20Server
  (params (Head :type Transform%20%28by%20ref%29) (Body :type Transform))
  ;[0.09375 0.09375 0.09375] Replicate
  (CallFunction|Multicast Head Body))

(event Custom|Multicast
  (params (Head :type Transform%20%28by%20ref%29) (Body :type Transform%20%28by%20ref%29))
  ;[0.09375 0.09375 0.09375] Replicate
  (Transformation|SetWorldTransform (Variables|Default|GetSM_Head) Head false false)
  (Transformation|SetWorldTransform (Variables|Default|GetSM_Body) Body false false))

(event Custom|Move
  (bind _camera (Variables|Default|GetCamera))
  (bind _returnvalue (Transformation|GetWorldTransform _camera))
  (if (Utilities|Operators|NotEqual(!=) (Transformation|GetWorldLocation (Variables|Default|GetCamera)) (Transformation|GetWorldLocation (Variables|/Script/Engine.Actor|GetRootComponent (Variables|Default|GetMarker))) 1.0)
    (Transformation|SetWorldTransform (Variables|Default|GetSM_Head) (Transformation|GetWorldTransform (Variables|Default|GetCamera)) false false)
    (Transformation|SetWorldTransform (Variables|Default|GetSM_Body) (Math|Transform|MakeTransform (.location _returnvalue) (Math|Rotator|MakeRotator 0.0 0.0 (.yaw (.rotation _returnvalue))) "1.000000,1.000000,1.000000") false false))
  (if (not (Ability|HasAuthority))
    (CallFunction|SendServer (Transformation|GetWorldTransform (Variables|Default|GetSM_Head)) (Transformation|GetWorldTransform (Variables|Default|GetSM_Body)))))

(event EventBeginPlay
  (Utilities|FlowControl|Sequence
    (:then_0
      (Variables|/AntilatencySDK/Blueprints/Samples/SceneComponents/BP_AltTrackerHmd.BP_AltTrackerHmd_C|SetHmdCamera (Variables|Default|GetBP_AltTrackerOculusHmd) (Variables|Default|GetCamera))
      (Development|ExecuteConsoleCommand "vr.PixelDensity 1.0" 0))
    (:then_1
      (bind _returnvalue (Actor|GetActorOfClass "/AntilatencySDK/Blueprints/Samples/Actors/BP_AltEnvironmentWithMarkers.BP_AltEnvironmentWithMarkers_C"))
      (Utilities|IsValid _returnvalue
        (:Is%20Valid
          (Variables|Default|SetMarker _returnvalue))))
    (:then_2
      (Utilities|Time|SetTimerbyEvent (delegate Custom|Move) 0.03 true))))

(event EventUnpossessed
  (params (OldController :type Controller%20Object%20Reference))
  ;[0.09375 0.09375 0.09375] Replicate
  (Actor|DestroyActor))

(fn ConstructionScript)